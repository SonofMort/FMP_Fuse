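; Interactable door that swings open and closed, or stays shut when locked.
; Interact casts the first player pawn to ThirdPersonPlayer and has it display a message if IsLocked is set.
; Otherwise it toggles IsOpen and plays or reverses the Door timeline, whose track lerps the static mesh's relative rotation through 80 degrees.
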(event `/Game/Interactables/Interact.Interact`
  (bind _asthird_person_player (cast `/Game/Gameplay/ThirdPersonPlayer` (`GameplayStatics.GetPlayerPawn` 0)))
  (if (`self.isLocked`)
    (`/Game/Gameplay/ThirdPersonPlayer.DisplayMessage` _asthird_person_player "This Door Is Locked!")
    (elif (`self.isOpen`)
      (set `self.isOpen` false)
      (bind (_direction _newtrack_0) (`Timeline|Door` :!via `Reverse` :!label _label)
        (:`Update`
          (`SceneComponent.K2_SetRelativeRotation` (`self.StaticMesh`) (`KismetMathLibrary.RLerp` (struct) (struct :`Yaw` -80.0) _newtrack_0) false false)))
      (else
        (set `self.isOpen` true)
        (goto _label)))))

(fn `UserConstructionScript`)